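; BP_RandomGen is a procedural tile generator that lays out a random grid of floor and wall pieces.
; The Construction Script sizes TileType to MaxX by MaxY, randomly sets each entry to 0 or 1, and adds a Floor or Wall mesh instance accordingly.
; Division and modulo by MaxY turn each flat array index into a grid position scaled by TileSize.
; The event graph holds only disabled placeholder events.
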(event EventBeginPlay)

(event Collision|EventActorBeginOverlap
  (params (OtherActor :type Actor%20Object%20Reference)))

(event EventTick
  (params (DeltaSeconds :type Float%20%28single-precision%29)))

(fn ConstructionScript
  (bind _tiletype (Variables|Default|GetTileType))
  (bind _tilesize (Variables|Default|GetTileSize))
  (bind _maxy (Variables|Default|GetMaxY))
  (Utilities|Array|Resize _tiletype (* (Variables|Default|GetMaxX) _maxy))
  (for (_array_element _array_index) _tiletype
    (Utilities|Array|SetArrayElem _tiletype _array_index (Math|Random|RandomIntegerinRange 0 1))
    (if (== _array_element 0)
      (Components|InstancedStaticMesh|AddInstance (Variables|Default|GetFloor) (Math|Conversions|ToTransform(Vector) (Math|Vector|MakeVector (Math|Conversions|ToFloat(Integer) (* (/ _array_index _maxy) _tilesize)) (Math|Conversions|ToFloat(Integer) (* (Math|Integer|%(Integer) _array_index _maxy) _tilesize)) 0.0)))
      (else
        (Components|InstancedStaticMesh|AddInstance (Variables|Default|GetWall) (Math|Conversions|ToTransform(Vector) (Math|Vector|MakeVector (Math|Conversions|ToFloat(Integer) (* (/ _array_index _maxy) _tilesize)) (Math|Conversions|ToFloat(Integer) (* (Math|Integer|%(Integer) _array_index _maxy) _tilesize)) 0.0)))))))